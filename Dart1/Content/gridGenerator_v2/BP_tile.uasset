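; BP_tile is a tile actor that positions itself within a grid by its Row and Column.
; Its Initalize function, if the owner is valid, attaches the tile to it, snapping location and rotation and keeping relative scale.
; It then offsets itself by Column and Row times the Tile component's box extent (half-size) in X and Y.
; The event graph and construction script are empty.
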(fn `Initalize`
  (bind _returnvalue (`self.GetOwner`))
  (`/Engine/EditorBlueprintResources/StandardMacros.IsValid` _returnvalue
    (:`Is Valid`
      (`self.K2_AttachToActor` _returnvalue "None" "SnapToTarget" "SnapToTarget" "KeepRelative")
      (`self.K2_SetActorRelativeLocation` (`KismetMathLibrary.MakeVector` (* (.x (`.BoxExtent` (`KismetSystemLibrary.GetComponentBounds` (`self.Tile`)))) (`self.column`)) (* (.y (`.BoxExtent` (`KismetSystemLibrary.GetComponentBounds` (`self.Tile`)))) (`self.row`)))))))

(fn `UserConstructionScript`)